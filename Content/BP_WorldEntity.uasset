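; BP_WorldEntity runs fade-in and fade-out transitions through two sequences, In and Out, and provides a sound hook for Sequencer.
; Each fade event binds to its sequence player's OnFinished before playing, and both completions print a debug message and call FadeFinished.
; A separate PlaySound event, grouped under Sequencer Events, plays the Audio from the start.
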(event `self.FadeHolderInBp`
  (add `MovieSceneSequencePlayer.OnFinished` (`ActorSequenceComponent.SequencePlayer` (`self.In`)) (delegate `CustomEvent`))
  (`ActorSequenceComponent.PlaySequence` (`self.In`)))

(event `CustomEvent`
  (`KismetSystemLibrary.PrintText` "Finished")
  (`self.FadeFinished` :!label _label))

(event `self.FadeHolderOutBp`
  (add `MovieSceneSequencePlayer.OnFinished` (`ActorSequenceComponent.SequencePlayer` (`self.Out`)) (delegate `OnFinished_Event`))
  (`ActorSequenceComponent.PlaySequence` (`self.Out`)))

(event `OnFinished_Event`
  (`KismetSystemLibrary.PrintText` "Finished")
  (goto _label))

(event `PlaySound`
  (`AudioComponent.Play` (`self.Audio`) 0.0))

(fn `UserConstructionScript`)